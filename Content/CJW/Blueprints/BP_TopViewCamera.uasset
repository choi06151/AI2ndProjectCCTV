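; BP_TopViewCamera is a top-view camera actor that follows the first-person player character from above.
; On BeginPlay it casts player character 0 to BP_FirstPersonCharacter and stores it as its target.
; Each tick, while the target is valid, it moves itself to the target's location plus a fixed offset along its own up vector, without sweeping.
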(event `self.ReceiveBeginPlay`
  (bind _asbp_first_person_character (cast `/Game/FirstPerson/Blueprints/BP_FirstPersonCharacter` (`GameplayStatics.GetPlayerCharacter` 0)))
  (set `self.Target` _asbp_first_person_character))

(event `self.ReceiveTick`
  (params (DeltaSeconds :type "Float (single-precision)"))
  (bind _target (`self.Target`))
  (`/Engine/EditorBlueprintResources/StandardMacros.IsValid` _target
    (:`Is Valid`
      (`self.K2_SetActorLocation` (+ (`self.K2_GetActorLocation` _target) (* (`self.GetActorUpVector`) 2000))))))

(fn `UserConstructionScript`)