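; Game mode for a murder-deduction game that marks the first third-person character as the murderer and runs timed kill turns.
; It opens paused on a start widget; GameStart unpauses and orders the first delayed kill, blinding the first-person player.
; NextTurn lifts the blind, then orders another kill or, past a kill-count limit, targets the player.
; CheckReliable compares detection data against the murderer's hat type to update the reliability UI.
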(event `self.ReceiveBeginPlay`
  (bind _output (`|GetArrayItem` (`self.PlayerList`)))
  ;[1 1 1] 플레이어의 정보를 가져와서 저장후, 살인자 한명 생성
  (bind _outactors (`GameplayStatics.GetAllActorsOfClass` "/Game/ThirdPerson/Blueprints/BP_ThirdPersonCharacter.BP_ThirdPersonCharacter_C"))
  (set `self.PlayerList` _outactors)
  (set `/Game/ThirdPerson/Blueprints/BP_ThirdPersonCharacter.IsMurderer` true _output)
  (set `self.Murder` _output)
  (bind _asbp_first_person_character (cast `/Game/FirstPerson/Blueprints/BP_FirstPersonCharacter` (`GameplayStatics.GetPlayerCharacter` 0)))
  (set `self.GamePlayer` _asbp_first_person_character)
  (bind _returnvalue (`|CreateWidget` "/Game/CJW/UI/WBP_GameStart.WBP_GameStart_C"))
  (`UserWidget.AddToViewport` _returnvalue 0)
  (`GameplayStatics.SetGamePaused` true))

(event `GameStart`
  (`GameplayStatics.SetGamePaused` false)
  (`Widget.RemoveFromParent` (stale `self.ReceiveBeginPlay` _returnvalue))
  (`KismetSystemLibrary.Delay` 10.0)
  (`self.Kill any one`))

(event `NextTurn`
  (`KismetSystemLibrary.Delay` 0.4)
  (`/Game/FirstPerson/Blueprints/BP_FirstPersonCharacter.EndKillingBlind` (`self.GamePlayer`))
  (`KismetSystemLibrary.Delay` 10.0)
  (if (<= (`/Game/ThirdPerson/Blueprints/BP_ThirdPersonCharacter.KillCount` (`self.Murder`)) 5)
    (`self.Kill any one`)
    (else
      (`/Game/ThirdPerson/Blueprints/BP_ThirdPersonCharacter.TargetIsPlayer` (`self.Murder`)))))

(event `GameEnd`)

(event `Kill any one`
  ;[1 1 1] 살인자한테 살인명령 내리기
  (`|ExecutionSequence`
    (:`then_0`
      (`/Game/ThirdPerson/Blueprints/BP_ThirdPersonCharacter.KillAnyOne` (`self.Murder`)))
    (:`then_1`
      (`KismetSystemLibrary.Delay` 0.4)
      (`/Game/FirstPerson/Blueprints/BP_FirstPersonCharacter.StartKillingBlind` (`self.GamePlayer`)))))

(event `self.UpdateReliabilityData`
  ;[1 1 1] UI 갱신(신뢰도)
  (bind _reliability (`self.CheckReliable`))
  (`TestWidget.UpdateReliabilityUI` (`self.TestUI`) _reliability))

(fn `CheckReliable`
  (returns (Reliability :type Boolean))
  (bind (_axe _bluecap _cowboyhat _dagger _gentlehat _greatsword _gun _laserblade _mariohat _santahat) (break `DetectionData` (`self.CurDetectionData`)))
  (switch `/Game/ENumList/EHatList` (`/Game/ThirdPerson/Blueprints/BP_ThirdPersonCharacter.HatType` (`self.Murder`))
    (:`NewEnumerator0`
      (if (> _cowboyhat 0)
        _
        (else
          (return false))))
    (:`NewEnumerator1`
      (if (> _bluecap 0)
        _
        (else
          (return false))))
    (:`NewEnumerator2`
      (if (> _gentlehat 0)
        _
        (else
          (return false))))
    (:`NewEnumerator3`
      (if (> _santahat 0)
        _
        (else
          (return false))))
    (:`NewEnumerator4`
      (if (> _mariohat 0)
        _
        (else
          (return false)))))
  (return true))

(fn `UserConstructionScript`)